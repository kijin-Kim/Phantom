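; BP_TestGameState is a test game state that relays player chat messages into the HUD chat window.
; The Chat function calls ServerChat, which formats sender and text into one line and passes it to MulticastChat.
; Outside dedicated servers, MulticastChat creates a WBP_ChatText widget, adds it to player 0's HUD ChatBox and scrolls to the end.
; It depends directly on BP_PhantomPlayerController's widget hierarchy, with a TODO to clean up dependencies.
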(event Custom|ServerChat
  (params (Sender :type Text) (Chat :type Text))
  ;[1 1 1] TODO : Dependency 정리하기
  (CallFunction|MulticastChat (Utilities|Text|FormatText "{Sender}: {Chat}" Sender Chat)))

(event Custom|MulticastChat
  (params (Chat :type Text))
  (bind _returnvalue (Game|GetPlayerController 0))
  ;[1 1 1] TODO : Dependency 정리하기
  (if (not (Networking|IsDedicatedServer))
    (bind _returnvalue_2 (UserInterface|CreateWidget "/Game/Widget/WBP_ChatText.WBP_ChatText_C" _returnvalue Chat))
    (bind _asbp_phantom_player_controller (Utilities|Casting|CastToBP_PhantomPlayerController _returnvalue))
    (Utilities|IsValid (Variables|/Game/Widget/WBP_ChatWindow.WBP_ChatWindow_C|GetChatBox (Variables|/Game/Widget/WBP_GameHUD.WBP_GameHUD_C|GetWBP_ChatWindow (Variables|/Game/PlayerCharacter/BP_PhantomPlayerController.BP_PhantomPlayerController_C|GetMainHUD _asbp_phantom_player_controller)))
      (:Is%20Valid
        (Widget|Panel|AddChild (Variables|/Game/Widget/WBP_ChatWindow.WBP_ChatWindow_C|GetChatBox (Variables|/Game/Widget/WBP_GameHUD.WBP_GameHUD_C|GetWBP_ChatWindow (Variables|/Game/PlayerCharacter/BP_PhantomPlayerController.BP_PhantomPlayerController_C|GetMainHUD _asbp_phantom_player_controller))) _returnvalue_2)
        (Class|ScrollBox|ScrolltoEnd (Variables|/Game/Widget/WBP_ChatWindow.WBP_ChatWindow_C|GetChatBox (Variables|/Game/Widget/WBP_GameHUD.WBP_GameHUD_C|GetWBP_ChatWindow (Variables|/Game/PlayerCharacter/BP_PhantomPlayerController.BP_PhantomPlayerController_C|GetMainHUD _asbp_phantom_player_controller))))))))

(event EventBeginPlay)

(event EventTick
  (params (DeltaSeconds :type Float%20%28single-precision%29)))

(fn ConstructionScript)

(fn Chat
  (params (Sender :type Text) (Chat :type Text))
  (CallFunction|ServerChat Sender Chat))