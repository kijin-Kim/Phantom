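; Player character Blueprint for the Phantom hero, supplying combat data through getters: attack, dodge and hit-react montages, motion warping and current target.
; Setters store combo window count and open state for the getters to return.
; BeginPlay hides bow and arrow bones, resets time dilation and applies the combat spring-arm offset.
; Walking and Running read HeroAction gameplay tags, but the camera-offset blending using them is disconnected, leaving Tick empty.
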(event EventBeginPlay
  (bind _combatspringarmpoint (Variables|Default|GetCombatSpringArmPoint))
  (bind _relativelocation (Variables|/Script/Engine.SceneComponent|GetRelativeLocation _combatspringarmpoint))
  (Components|SkinnedMesh|HideBonebyName (Variables|Character|GetMesh) "bow_base" "PBO_None")
  (Components|SkinnedMesh|HideBonebyName (Variables|Character|GetMesh) "arrow_nock" "PBO_None")
  (Utilities|Time|SetGlobalTimeDilation 1.0)
  (Variables|Default|SetCameraSocketOffset (Variables|/Script/Engine.SceneComponent|GetRelativeLocation (Variables|Default|GetWalkingSpringArmPoint)))
  (Variables|Default|SetCameraSocketOffset _relativelocation)
  (Variables|/Script/Engine.SpringArmComponent|SetSocketOffset (Variables|Default|GetCameraBoom) _relativelocation))

(event EventSetAttackSequenceComboCount
  (params (Count :type Integer))
  (Variables|Default|SetComboWindowCount Count))

(event EventSetComboWindowOpened
  (params (bIsOpened :type Boolean))
  (Variables|Default|SetComboWindowOpened bIsOpened))

(event EventTick
  (params (DeltaSeconds :type Float%20%28single-precision%29))
  (Utilities|FlowControl|Sequence))

(fn ConstructionScript)

(fn GetDodgeMontage
  (return "/Game/PrivateAsset/Phantom/Sword/AM_Phantom_Sword_Roll_F_0_Seq_Montage.AM_Phantom_Sword_Roll_F_0_Seq_Montage"))

(fn Walking
  (return (not (GameplayTags|HasAnyMatchingGameplayTags (Variables|Default|GetHeroActionComponent) (Utilities|Struct|MakeGameplayTagContainer (Utilities|Array|MakeArray "(TagName=\"HeroAction.Run\")" "(TagName=\"HeroAction.Sprint\")"))))))

(fn Running
  (return (GameplayTags|HasMatchingGameplayTag (Variables|Default|GetHeroActionComponent) "(TagName=\"HeroAction.Run\")")))

(fn GetAttackMontages
  (return (Utilities|Array|MakeArray "/Game/PrivateAsset/Phantom/GhostSamurai/AM_Phantom_Attack01.AM_Phantom_Attack01" "/Game/PrivateAsset/Phantom/GhostSamurai/AM_Phantom_GS_APose_Attack02.AM_Phantom_GS_APose_Attack02")))

(fn GetAttackSequenceComboCount
  (return (Variables|Default|GetComboWindowCount)))

(fn GetComboWindowOpened
  (return (Variables|Default|GetComboWindowOpened)))

(fn GetMotionWarpingComponent
  (return (Variables|Default|GetMotionWarping)))

(fn GetTargetedActor
  (return (Variables|Default|GetCurrentTargeted)))

(fn GetHitReactMontage
  (return "/Game/PrivateAsset/Phantom/GhostSamurai/AM_Phantom_APose_Hit.AM_Phantom_APose_Hit"))