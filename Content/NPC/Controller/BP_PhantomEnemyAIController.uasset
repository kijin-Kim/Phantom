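; AI controller for BP_PhantomEnemy that records perceived actors as invaders in the Blackboard.
; Perception updates within a height band set the PrivateInvaderName key, also filling InvaderName when its vector-value check reports unset.
; The actor is also stored as the pawn's PrivateInvader if it is a PhantomCharacterBase.
; Forgetting a target clears the pawn's PrivateInvader and its Blackboard key, leaving InvaderName untouched.
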(event OnTargetPerceptionUpdated(PerceptionComponent)
  (params (Actor :type Actor%20Object%20Reference) (Stimulus :type AI%20Stimulus%20Structure))
  (if (< (Math|Float|Absolute(Float) (- (.z (Transformation|GetActorLocation Actor)) (.z (Transformation|GetActorLocation (Pawn|GetControlledPawn))))) 2e+02)
    (if (Class|BlackboardComponent|IsVectorValueSet (Variables|Default|GetBlackboard) (Variables|Default|GetInvader%20Name))
      (AI|Components|Blackboard|SetValueasObject (Variables|Default|GetBlackboard) (Variables|Default|GetPrivate%20Invader%20Name) Actor)
      (bind _asbp_phantom_enemy (Utilities|Casting|CastToBP_PhantomEnemy (Pawn|GetControlledPawn)))
      (bind _asphantom_character_base (Utilities|Casting|CastToPhantomCharacterBase Actor))
      (Variables|/Script/Phantom.PhantomEnemy|SetPrivateInvader _asbp_phantom_enemy _asphantom_character_base)
      (else
        (AI|Components|Blackboard|SetValueasObject (Variables|Default|GetBlackboard) (Variables|Default|GetInvader%20Name) Actor)
        (AI|Components|Blackboard|SetValueasObject (Variables|Default|GetBlackboard) (Variables|Default|GetPrivate%20Invader%20Name) Actor)
        (bind _asbp_phantom_enemy_2 (Utilities|Casting|CastToBP_PhantomEnemy (Pawn|GetControlledPawn)))
        (bind _asphantom_character_base_2 (Utilities|Casting|CastToPhantomCharacterBase Actor))
        (Variables|/Script/Phantom.PhantomEnemy|SetPrivateInvader _asbp_phantom_enemy_2 _asphantom_character_base_2)))))

(event OnTargetPerceptionForgotten(PerceptionComponent)
  (params (Actor :type Actor%20Object%20Reference))
  (bind _asbp_phantom_enemy (Utilities|Casting|CastToBP_PhantomEnemy (Pawn|GetControlledPawn)))
  (Variables|/Script/Phantom.PhantomEnemy|SetPrivateInvader _asbp_phantom_enemy 0)
  (AI|Components|Blackboard|ClearValue (Variables|Default|GetBlackboard) (Variables|Default|GetPrivate%20Invader%20Name)))

(event EventBeginPlay)

(fn ConstructionScript)