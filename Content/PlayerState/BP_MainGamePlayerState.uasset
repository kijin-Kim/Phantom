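; Main game player state that relays text chat messages to players' HUD chat windows.
; ServerChat formats the sender and message into one line and passes it to MulticastChat.
; MulticastChat skips dedicated servers, creates a WBP_ChatText widget, appends it to the chat box in the local BP_PhantomPlayerController's MainHUD and scrolls to the end.
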(event Custom|ServerChat
  (params (Sender :type Text) (Chat :type Text))
  (CallFunction|MulticastChat (Utilities|Text|FormatText "[{Sender}] : {Chat}" Sender Chat)))

(event Custom|MulticastChat
  (params (FormatedChat :type Text))
  (bind _returnvalue (Game|GetPlayerController 0))
  (if (not (Networking|IsDedicatedServer))
    (bind _returnvalue_2 (UserInterface|CreateWidget "/Game/UI/Widget/WBP_ChatText.WBP_ChatText_C" _returnvalue FormatedChat))
    (bind _asbp_phantom_player_controller (Utilities|Casting|CastToBP_PhantomPlayerController _returnvalue))
    (Utilities|IsValid (Variables|/Game/UI/Widget/WBP_ChatWindow.WBP_ChatWindow_C|GetChatBox (Variables|/Game/UI/Widget/WBP_GameHUD.WBP_GameHUD_C|GetWBP_ChatWindow (Variables|/Game/PlayerCharacter/BP_PhantomPlayerController.BP_PhantomPlayerController_C|GetMainHUD _asbp_phantom_player_controller)))
      (:Is%20Valid
        (Widget|Panel|AddChild (Variables|/Game/UI/Widget/WBP_ChatWindow.WBP_ChatWindow_C|GetChatBox (Variables|/Game/UI/Widget/WBP_GameHUD.WBP_GameHUD_C|GetWBP_ChatWindow (Variables|/Game/PlayerCharacter/BP_PhantomPlayerController.BP_PhantomPlayerController_C|GetMainHUD _asbp_phantom_player_controller))) _returnvalue_2)
        (Class|ScrollBox|ScrolltoEnd (Variables|/Game/UI/Widget/WBP_ChatWindow.WBP_ChatWindow_C|GetChatBox (Variables|/Game/UI/Widget/WBP_GameHUD.WBP_GameHUD_C|GetWBP_ChatWindow (Variables|/Game/PlayerCharacter/BP_PhantomPlayerController.BP_PhantomPlayerController_C|GetMainHUD _asbp_phantom_player_controller))))))))

(event EventBeginPlay)

(event EventTick
  (params (DeltaSeconds :type Float%20%28single-precision%29)))

(fn ConstructionScript)