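; BP_PhantomPlayerController is a player controller that creates the game HUD for the local player.
; On BeginPlay, if the controller is local and not on a dedicated server, it creates WBP_GameHUD, stores it as MainHUD and adds it to the viewport.
; An unconnected FlipFlop for toggling the mouse cursor and UI-only or game-only input mode never runs.
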(event EventBeginPlay
  (if (and (Pawn|IsLocalPlayerController) (not (Networking|IsDedicatedServer)))
    (bind _returnvalue (UserInterface|CreateWidget "/Game/Widget/WBP_GameHUD.WBP_GameHUD_C"))
    (bind _output_get (Variables|Default|SetMainHUD _returnvalue))
    (UserInterface|Viewport|AddtoViewport _output_get 0)))

(fn ConstructionScript)